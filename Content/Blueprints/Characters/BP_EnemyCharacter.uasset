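; Enemy character Blueprint that fades its mesh in and out of invisibility through material effects.
; BeginPlay and the turn-on event put a dynamic instance of the enemy invisibility material on the mesh's first slot.
; Separate on and off timelines drive its Invisibility scalar parameter, and the off timeline swaps in a Mutant_M instance when finished.
; The UpdateMaterial function is an unimplemented stub.
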(event `self.ReceiveBeginPlay`
  (bind _returnvalue (`PrimitiveComponent.CreateDynamicMaterialInstance` (`self.Mesh`) 0 "/Game/Materials/CharacterMaterials/M_EnemyMatInstance.M_EnemyMatInstance" "None"))
  (set `self.Invisible material` _returnvalue))

(event `self.TurnInvisibilityOn`
  (bind _returnvalue (`PrimitiveComponent.CreateDynamicMaterialInstance` (`self.Mesh`) 0 "/Game/Materials/CharacterMaterials/M_EnemyMatInstance.M_EnemyMatInstance" "None"))
  (set `self.Invisible material` _returnvalue)
  (bind (_direction _newtrack_0) (`Timeline|Invisibility on animation`)
    (:`Update`
      (`MaterialInstanceDynamic.SetScalarParameterValue` (`self.Invisible material`) "Invisibility" _newtrack_0))))

(event `self.TurnInvisibilityOff`
  (bind (_direction _newtrack_0) (`Timeline|Invisibility off animation`)
    (:`Update`
      (`MaterialInstanceDynamic.SetScalarParameterValue` (`self.Invisible material`) "Invisibility" _newtrack_0))
    (:`Finished`
      (`PrimitiveComponent.CreateDynamicMaterialInstance` (`self.Mesh`) 0 "/Game/Assets/Test/mutant_M.mutant_M" "None"))))

(fn `Update material`
  (params (Value :type "Float (double-precision)")))

(fn `UserConstructionScript`)