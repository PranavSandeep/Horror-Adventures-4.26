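; Player character Blueprint with camera pitch, forward-axis movement, Shift sprint and a proximity warning for an enemy.
; Tick checks distance to the first enemy found at BeginPlay, using a resettable DoOnce to show an alert widget and start a looping heartbeat timer.
; Leaving range clears both.
; Any damage is fatal: the camera attaches to the head socket, input is disabled, and the actor is destroyed after a delay.
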(event `self.ReceiveBeginPlay`
  (bind _outactors (`GameplayStatics.GetAllActorsOfClass` "/Game/Blueprints/Characters/BP_EnemyCharacter.BP_EnemyCharacter_C"))
  (bind _output (`|GetArrayItem` _outactors))
  (`/Engine/EditorBlueprintResources/StandardMacros.IsValid` _output
    (:`Is Valid`
      (set `self.Enemy` _output))))

(event `self.ReceiveAnyDamage`
  (params (Damage :type "Float (single-precision)") (DamageType :type "DamageType Object Reference") (InstigatedBy :type "Controller Object Reference") (DamageCauser :type "Actor Object Reference"))
  ;[1 1 1] Death
  (`SceneComponent.K2_AttachToComponent` (`self.Camera`) (`self.Mesh`) "Head" "KeepWorld" "KeepRelative" "KeepRelative" true)
  (set `self.Is Ded?` true)
  (`self.DisableInput` (`GameplayStatics.GetPlayerController` 0))
  (`KismetSystemLibrary.Delay` 2.8)
  (`self.DetachFromControllerPendingDestroy`)
  (`self.K2_DestroyActor`))

(event `InputAxisKey|MouseY`
  (params (AxisValue :type "Float (single-precision)"))
  ;[1 1 1] Mouse Controls
  (`SceneComponent.K2_AddLocalRotation` (`self.Camera`) (`KismetMathLibrary.MakeRotator` 0.0 AxisValue) false false))

(event `self.ReceiveTick`
  (params (DeltaSeconds :type "Float (single-precision)"))
  (bind _enemy (`self.Enemy`))
  (`/Engine/EditorBlueprintResources/StandardMacros.IsValid` _enemy
    (:`Is Valid`
      (if (<= (`KismetMathLibrary.Vector_Distance` (`self.K2_GetActorLocation`) (`self.K2_GetActorLocation` _enemy)) 1000.0)
        (`/Engine/EditorBlueprintResources/StandardMacros.DoOnce` false :!label _label
          (:`Completed`
            (`self.AlertPlayerIfEnemyIsNear`)))
        (else
          (`self.ClearHeartbeatTimerHandle` (`self.Heart Beat Timer Handle`))
          (goto _label :!via `Reset`))))))

(event `self.AlertPlayerIfEnemyIsNear`
  (bind _returnvalue (`GameplayStatics.GetPlayerController` 0))
  ;[1 1 1] Alert Player
  (set `self.Is Near Enemy?` true)
  (bind _returnvalue_2 (`|CreateWidget` "/Game/UI/WBP_AlertPlayer.WBP_AlertPlayer_C" _returnvalue))
  (set `self.Alert UI` _returnvalue_2)
  (`UserWidget.AddToViewport` _returnvalue_2 0)
  (`self.Play Heartbeat Sound` (`self.K2_GetActorLocation` _returnvalue))
  (bind _returnvalue_3 (`KismetSystemLibrary.K2_SetTimer` null "Play Heartbeat" 1.5 true))
  (set `self.Heart Beat Timer Handle` _returnvalue_3))

(event `self.ClearHeartbeatTimerHandle`
  (params (HeartbeatHandle :type "TimerHandle Structure"))
  (bind _alert_ui (`self.Alert UI`))
  ;[1 1 1] Stop Alerting Player
  (`KismetSystemLibrary.K2_ClearAndInvalidateTimerHandle` HeartbeatHandle)
  (`/Engine/EditorBlueprintResources/StandardMacros.IsValid` _alert_ui
    (:`Is Valid`
      (`Widget.RemoveFromParent` _alert_ui))))

(event `Key|LeftShift`
  (params (Key :type "Key Structure"))
  (bind _charactermovement (`self.CharacterMovement`))
  (:`Pressed`
    (set `CharacterMovementComponent.MaxWalkSpeed` 1000.0 _charactermovement))
  (:`Released`
    (set `CharacterMovementComponent.MaxWalkSpeed` 580.0 _charactermovement)))

(event `Key|Seven`
  (params (Key :type "Key Structure"))
  (:`Pressed`
    (`self.TurnOffLight` self)))

(event `InputAxis|Test`
  (params (AxisValue :type "Float (single-precision)"))
  (`self.AddMovementInput` (`KismetMathLibrary.GetForwardVector` (`SceneComponent.K2_GetComponentRotation` (`self.Camera`))) AxisValue))

(fn `Play Heartbeat`
  (`GameplayStatics.PlaySoundAtLocation` "/Game/SFX/Heartbeat_single_.Heartbeat_single_" (`self.K2_GetActorLocation`) (struct) 1.0 1.0 0.0 null null null))

(fn `Play Heartbeat Sound`
  (params (Location :type "Vector Structure"))
  (`GameplayStatics.PlaySoundAtLocation` "/Game/SFX/Heartbeat_single_.Heartbeat_single_" (`self.K2_GetActorLocation`) (struct) 1.0 1.0 0.0 null null null))

(fn `UserConstructionScript`)